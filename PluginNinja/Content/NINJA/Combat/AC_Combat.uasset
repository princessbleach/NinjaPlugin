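; Actor component that handles sword combat for BP_ThirdPersonCharacter, covering weapon equip, storage and a two-hit slash combo.
; Attack input requires an equipped sword and the IsAttacking flag, set through CallAttacking, then plays a slash montage selected by ComboCount.
; The combo counter wraps after the second slash or resets through a retriggerable delay.
; EquipWeapon spawns BP_Sword on the mesh's SwordSocket, and StoreWeapon destroys it.
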(event `self.ReceiveBeginPlay`
  ; CharRef
  (bind _asbp_third_person_character (cast `/Game/NINJA/Ninja/BP_ThirdPersonCharacter` (`self.GetOwner`)))
  (set `self.CharRef` _asbp_third_person_character))

(event `EnhancedInput|/Game/Input/Actions/IA_Attack`
  (params (ActionValue :type Boolean) (ElapsedSeconds :type "Float (double-precision)") (TriggeredSeconds :type "Float (double-precision)") (InputAction :type "InputAction Object Reference" :default "/Game/Input/Actions/IA_Attack.IA_Attack"))
  (bind _combocount (`self.ComboCount`))
  ; Combo
  (:`Triggered`
    (if (`/Game/NINJA/Ninja/BP_ThirdPersonCharacter.SwordEquipped?` (`self.CharRef`))
      (if (`self.IsAttacking?`)
        (`|PlayMontage` (`Character.Mesh` (`self.CharRef`)) (select `int` (`self.ComboCount`) :`0` "/Game/NINJA/Animations/AM_Slash1.AM_Slash1" :`1` "/Game/NINJA/Animations/AM_Slash2.AM_Slash2" :!type "AnimMontage Object Reference")
          (:`then`
            (`self.SetComponentTickEnabled` true)
            (`/Engine/EditorBlueprintResources/StandardMacros.IncrementInt` _combocount
              (:`  `
                (if (> _combocount 1)
                  (set `self.ComboCount` 0)
                  (else
                    (`KismetSystemLibrary.RetriggerableDelay` 2.0)
                    (set `self.ComboCount` 0)))))))))))

(event `/Game/NINJA/Combat/BPI_COmponent.CallAttacking`
  (params (Attacking :type Boolean))
  ; Combo
  (set `self.IsAttacking?` Attacking))

(event `EquipWeapon`
  (bind _returnvalue (`self.GetOwner`))
  ; EquipSword
  (bind _returnvalue_2 (`|SpawnActorFromClass` "/Game/NINJA/Sword/BP_Sword.BP_Sword_C" (`Actor.GetTransform` _returnvalue) "Undefined" "MultiplyWithRoot" null null))
  (bind _output_get (set `self.SwordRef` _returnvalue_2))
  (bind _asbp_third_person_character (cast `/Game/NINJA/Ninja/BP_ThirdPersonCharacter` _returnvalue))
  (`Actor.K2_AttachToComponent` _output_get (`Character.Mesh` _asbp_third_person_character) "SwordSocket" "SnapToTarget" "SnapToTarget" "SnapToTarget" true))

(event `StoreWeapon`
  ; Store Weapon
  (`Actor.K2_DestroyActor` (`self.SwordRef`)))